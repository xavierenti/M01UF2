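; BP_Targets is a moving target actor that is destroyed when a first-person projectile hits it.
; Each Tick it sweeps forward along its Arrow component's direction, scaled by the Veloidad speed and delta time.
; On overlap it destroys the projectile and itself, then calls AddPoints only if that same overlapping actor also casts to BP_FirstPersonCharacter, so projectile hits likely never score.
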(event EventTick
  (params (DeltaSeconds :type Float%20%28single-precision%29))
  ;[0.05098 0.05098 0.05098] Dar velocidad al objeto
  (Transformation|AddActorWorldOffset (* (* DeltaSeconds (Variables|Default|GetVeloidad)) (Math|Vector|GetForwardVector (Variables|Default|GetArrow))) true))

(event Collision|EventActorBeginOverlap
  (params (OtherActor :type Actor%20Object%20Reference))
  ;[0.05098 0.05098 0.05098] Destruccion de objetos y Suma de puntos
  (bind _asbp_first_person_projectile (Utilities|Casting|CastToBP_FirstPersonProjectile OtherActor))
  (Actor|DestroyActor _asbp_first_person_projectile)
  (Actor|DestroyActor)
  (bind _asbp_first_person_character (Utilities|Casting|CastToBP_FirstPersonCharacter OtherActor))
  (Default|AddPoints _asbp_first_person_character))

(fn ConstructionScript)