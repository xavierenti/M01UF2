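; BP_Spawner is a spawner actor that creates BP_Targets actors at a set position and rotation once the GameStart event sets GameStarted.
; While started, Tick spawns a target every frame if CantidadDeTiros is positive, otherwise clears the flag.
; Each spawn feeds a Tiempotiro Delay that loops back to spawning without rechecking either condition.
; CantidadDeTiros is never decremented in this Blueprint.
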(event Custom|GameStart
  ;[0.05098 0.05098 0.05098] Recibir spauner Starter
  (Variables|Default|SetGame%20started true))

(event EventBeginPlay)

(event Collision|EventActorBeginOverlap
  (params (OtherActor :type Actor%20Object%20Reference)))

(event EventTick
  (params (DeltaSeconds :type Float%20%28single-precision%29))
  ;[0.05098 0.05098 0.05098] Comprobacion de spawn / Si se espawnea y quando se acaba
  (if (Variables|Default|GetGame%20started)
    (if (> (Variables|Default|GetCantidad%20de%20tiros) 0.0)
      (Game|SpawnActorfromClass "/Game/Spawner/BP_Targets.BP_Targets_C" (Math|Transform|MakeTransform (Variables|Default|GetPosition) (Variables|Default|GetRotation) "1.000000,1.000000,1.000000") "Undefined" "MultiplyWithRoot" 0 1e+02 0 :!label _label)
      (Utilities|FlowControl|Delay (Variables|Default|GetTiempotiro))
      (goto _label)
      (else
        (Variables|Default|SetGame%20started false)))))

(fn ConstructionScript)